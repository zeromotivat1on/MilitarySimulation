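; BP_VehiclePath is a spline path for the vehicle convoy that answers position and progress queries.
; GetClosestLocationToVehiclePath projects a vehicle's world location onto the spline, then returns the world point a given distance offset along it, usable as a look-ahead target.
; GetDrivenDistance turns a location into distance along the spline and adds the full spline length per non-negative lap, giving cumulative distance across laps.
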(fn `GetClosestLocationToVehiclePath`
  (params (VehicleLocation :type "Vector Structure") (SplineOffset :type "Float (double-precision)"))
  (returns (SteerLocation :type "Vector Structure"))
  (bind _spline (`self.Spline`))
  (return (`SplineComponent.GetLocationAtDistanceAlongSpline` _spline (+ (`SplineComponent.GetDistanceAlongSplineAtLocation` _spline VehicleLocation "World") SplineOffset) "World")))

(fn `GetDrivenDistance`
  (params (Location :type "Vector Structure") (Lap :type Integer))
  (returns (PathDistance :type "Float (double-precision)"))
  (bind _spline (`self.Spline`))
  (return (+ (`SplineComponent.GetDistanceAlongSplineAtLocation` _spline Location "World") (* (`SplineComponent.GetSplineLength` _spline) (`KismetMathLibrary.Max` Lap)))))

(fn `UserConstructionScript`)