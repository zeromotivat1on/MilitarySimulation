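; BP_Player is a player Blueprint that acts as a keyboard test controller for a military vehicle convoy.
; On BeginPlay it finds the BP_MilitaryVehicleConvoy actor in the level and stores the reference.
; Number keys explode individual convoy vehicles by index, while letter keys spawn the convoy, destroy it or toggle its debug display through a FlipFlop.
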(event `self.ReceiveBeginPlay`
  (bind _returnvalue (`GameplayStatics.GetActorOfClass` "/Game/VehicleConvoy/BP_MilitaryVehicleConvoy.BP_MilitaryVehicleConvoy_C"))
  (set `self.MilitaryConvoy` _returnvalue))

(event `Key|One`
  (params (Key :type "Key Structure"))
  (:`Pressed`
    (`/Game/VehicleConvoy/BP_MilitaryVehicleConvoy.ExplodeVehicle` (`self.MilitaryConvoy`) 0)))

(event `Key|Two`
  (params (Key :type "Key Structure"))
  (:`Pressed`
    (`/Game/VehicleConvoy/BP_MilitaryVehicleConvoy.ExplodeVehicle` (`self.MilitaryConvoy`) 1)))

(event `Key|Three`
  (params (Key :type "Key Structure"))
  (:`Pressed`
    (`/Game/VehicleConvoy/BP_MilitaryVehicleConvoy.ExplodeVehicle` (`self.MilitaryConvoy`) 2)))

(event `Key|Four`
  (params (Key :type "Key Structure"))
  (:`Pressed`
    (`/Game/VehicleConvoy/BP_MilitaryVehicleConvoy.ExplodeVehicle` (`self.MilitaryConvoy`) 3)))

(event `Key|Five`
  (params (Key :type "Key Structure"))
  (:`Pressed`
    (`/Game/VehicleConvoy/BP_MilitaryVehicleConvoy.ExplodeVehicle` (`self.MilitaryConvoy`) 4)))

(event `Key|T`
  (params (Key :type "Key Structure"))
  (:`Pressed`
    (`VehicleConvoy.Spawn` (`self.MilitaryConvoy`))))

(event `Key|R`
  (params (Key :type "Key Structure"))
  (:`Pressed`
    (`VehicleConvoy.DestroyConvoy` (`self.MilitaryConvoy`))))

(event `Key|Y`
  (params (Key :type "Key Structure"))
  (:`Pressed`
    (bind _isa (`/Engine/EditorBlueprintResources/StandardMacros.FlipFlop`)
      (:`A`
        _)
      (:`B`
        _))
    (`/Game/VehicleConvoy/BP_MilitaryVehicleConvoy.SetShowDebug` (`self.MilitaryConvoy`) _isa)))

(fn `UserConstructionScript`)